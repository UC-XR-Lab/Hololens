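; BP_MaterialOverride, part of an architectural section tool, swaps materials on chosen static mesh actors to one override material.
; The construction script builds the active list from all static mesh actors or user-picked and tagged ones, moving meshes excluded by list or tag into OtherMeshes.
; ReplaceMaterials overrides every slot and optionally hides OtherMeshes.
; ResetMaterials clears the slot overrides and, with the same option, shows them again.
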(event `ReplaceMaterials`
  (for _array_element (`self.ActiveMeshes`)
    (bind _staticmeshcomponent (`StaticMeshActor.StaticMeshComponent` _array_element))
    (for (_ _array_index) (`MeshComponent.GetMaterials` _staticmeshcomponent)
      (`PrimitiveComponent.SetMaterial` _staticmeshcomponent _array_index (`self.MaterialOverride`))
      (if (`self.HideOthers`)
        (for _array_element_2 (`self.OtherMeshes`)
          (`SceneComponent.SetVisibility` (`StaticMeshActor.StaticMeshComponent` _array_element_2) false false))))))

(event `ResetMaterials`
  (for _array_element (`self.ActiveMeshes`)
    (bind _staticmeshcomponent (`StaticMeshActor.StaticMeshComponent` _array_element))
    (for (_ _array_index) (`MeshComponent.GetMaterials` _staticmeshcomponent)
      (`PrimitiveComponent.SetMaterial` _staticmeshcomponent _array_index null)
      (if (`self.HideOthers`)
        (for _array_element_2 (`self.OtherMeshes`)
          (`SceneComponent.SetVisibility` (`StaticMeshActor.StaticMeshComponent` _array_element_2) true false))))))

(fn `UserConstructionScript`
  (bind _excludetags (`self.ExcludeTags`))
  (bind _includetags (`self.IncludeTags`))
  ;[1 1 1] Initial Mesh Array - either All or User Selected
  (if (`self.OverrideAll `)
    (bind _outactors (`GameplayStatics.GetAllActorsOfClass` "/Script/Engine.StaticMeshActor"))
    (set `self.ActiveMeshes` _outactors)
    (`|ExecutionSequence` :!label _label
      (:`then_0`
        ;[1 1 1] Remove User Specified Meshes
        (if (> (`KismetArrayLibrary.Array_Length` (`self.ExcludeMeshes`)) 0)
          (for _array_element (`self.ExcludeMeshes`)
            (`KismetArrayLibrary.Array_Add` (`self.OtherMeshes`) _array_element))))
      (:`then_1`
        ;[1 1 1] Remove Meshes with Specified Tags
        (if (> (`KismetArrayLibrary.Array_Length` _excludetags) 0)
          (for _array_element_2 _excludetags
            (bind _outactors_2 (`GameplayStatics.GetAllActorsWithTag` _array_element_2))
            (for _array_element_3 _outactors_2
              (bind _asstatic_mesh_actor (cast `StaticMeshActor` _array_element_3))
              (`KismetArrayLibrary.Array_Add` (`self.OtherMeshes`) _asstatic_mesh_actor)))))
      (:`then_2`
        ;[1 1 1] Remove Meshes
        (for _array_element_4 (`self.OtherMeshes`)
          (`KismetArrayLibrary.Array_RemoveItem` (`self.ActiveMeshes`) _array_element_4))))
    (else
      (set `self.ActiveMeshes` (`self.IncludeMeshes`))
      ;[1 1 1] Add Meshes with Specified Tags
      (if (> (`KismetArrayLibrary.Array_Length` _includetags) 0)
        (for _array_element_5 _includetags
          (bind _outactors_3 (`GameplayStatics.GetAllActorsWithTag` _array_element_5))
          (for _array_element_6 _outactors_3
            (bind _asstatic_mesh_actor_2 (cast `StaticMeshActor` _array_element_6))
            (`KismetArrayLibrary.Array_Add` (`self.ActiveMeshes`) _asstatic_mesh_actor_2)
            (goto _label)))))))