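; Box cutout actor for the architectural section tool, feeding a box volume to materials through the MPC_ArchitecturalParameters collection.
; Four corner components give world positions, written as BoxPointA–D on construction when enabled and on Tick when UpdateEveryFrame is set.
; ToggleBox and InvertBox flags are pushed as scalars, and ToggleBoxOnOff flips the box at runtime.
; The construction script also sets the preview cube's opacity via a dynamic material instance.
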(event `self.ReceiveBeginPlay`
  (if (`self.ToggleBox`)
    (`KismetMaterialLibrary.SetScalarParameterValue` "/Game/ArchitectualSectionTool/Materials/MPC_ArchitecturalParameters.MPC_ArchitecturalParameters" "ToggleBox" 1.0)
    (if (`self.InvertBox`)
      (`KismetMaterialLibrary.SetScalarParameterValue` "/Game/ArchitectualSectionTool/Materials/MPC_ArchitecturalParameters.MPC_ArchitecturalParameters" "InvertBox" 1.0)
      (else
        (`KismetMaterialLibrary.SetScalarParameterValue` "/Game/ArchitectualSectionTool/Materials/MPC_ArchitecturalParameters.MPC_ArchitecturalParameters" "InvertBox")))
    (else
      (`KismetMaterialLibrary.SetScalarParameterValue` "/Game/ArchitectualSectionTool/Materials/MPC_ArchitecturalParameters.MPC_ArchitecturalParameters" "ToggleBox"))))

(event `self.ReceiveTick`
  (params (DeltaSeconds :type "Float (single-precision)"))
  (if (`self.UpdateEveryFrame`)
    (`KismetMaterialLibrary.SetVectorParameterValue` "/Game/ArchitectualSectionTool/Materials/MPC_ArchitecturalParameters.MPC_ArchitecturalParameters" "BoxPointA" (`KismetMathLibrary.Conv_VectorToLinearColor` (`SceneComponent.K2_GetComponentLocation` (`self.BoxA`))))
    (`KismetMaterialLibrary.SetVectorParameterValue` "/Game/ArchitectualSectionTool/Materials/MPC_ArchitecturalParameters.MPC_ArchitecturalParameters" "BoxPointB" (`KismetMathLibrary.Conv_VectorToLinearColor` (`SceneComponent.K2_GetComponentLocation` (`self.BoxB`))))
    (`KismetMaterialLibrary.SetVectorParameterValue` "/Game/ArchitectualSectionTool/Materials/MPC_ArchitecturalParameters.MPC_ArchitecturalParameters" "BoxPointC" (`KismetMathLibrary.Conv_VectorToLinearColor` (`SceneComponent.K2_GetComponentLocation` (`self.BoxC`))))
    (`KismetMaterialLibrary.SetVectorParameterValue` "/Game/ArchitectualSectionTool/Materials/MPC_ArchitecturalParameters.MPC_ArchitecturalParameters" "BoxPointD" (`KismetMathLibrary.Conv_VectorToLinearColor` (`SceneComponent.K2_GetComponentLocation` (`self.BoxD`))))))

(event `ToggleBoxOnOff`
  (if (`self.ToggleBox`)
    (`KismetMaterialLibrary.SetScalarParameterValue` "/Game/ArchitectualSectionTool/Materials/MPC_ArchitecturalParameters.MPC_ArchitecturalParameters" "ToggleBox")
    (set `self.ToggleBox` false)
    (else
      (`KismetMaterialLibrary.SetScalarParameterValue` "/Game/ArchitectualSectionTool/Materials/MPC_ArchitecturalParameters.MPC_ArchitecturalParameters" "ToggleBox" 1.0)
      (set `self.ToggleBox` true))))

(fn `UserConstructionScript`
  (bind _returnvalue (`PrimitiveComponent.CreateDynamicMaterialInstance` (`self.Cube`) 0 null "None"))
  (`MaterialInstanceDynamic.SetScalarParameterValue` _returnvalue "Opacity" (`self.Opacity`))
  (if (`self.ToggleBox`)
    (`KismetMaterialLibrary.SetScalarParameterValue` "/Game/ArchitectualSectionTool/Materials/MPC_ArchitecturalParameters.MPC_ArchitecturalParameters" "ToggleBox" 1.0)
    (`KismetMaterialLibrary.SetVectorParameterValue` "/Game/ArchitectualSectionTool/Materials/MPC_ArchitecturalParameters.MPC_ArchitecturalParameters" "BoxPointA" (`KismetMathLibrary.Conv_VectorToLinearColor` (`SceneComponent.K2_GetComponentLocation` (`self.BoxA`))))
    (`KismetMaterialLibrary.SetVectorParameterValue` "/Game/ArchitectualSectionTool/Materials/MPC_ArchitecturalParameters.MPC_ArchitecturalParameters" "BoxPointB" (`KismetMathLibrary.Conv_VectorToLinearColor` (`SceneComponent.K2_GetComponentLocation` (`self.BoxB`))))
    (`KismetMaterialLibrary.SetVectorParameterValue` "/Game/ArchitectualSectionTool/Materials/MPC_ArchitecturalParameters.MPC_ArchitecturalParameters" "BoxPointC" (`KismetMathLibrary.Conv_VectorToLinearColor` (`SceneComponent.K2_GetComponentLocation` (`self.BoxC`))))
    (`KismetMaterialLibrary.SetVectorParameterValue` "/Game/ArchitectualSectionTool/Materials/MPC_ArchitecturalParameters.MPC_ArchitecturalParameters" "BoxPointD" (`KismetMathLibrary.Conv_VectorToLinearColor` (`SceneComponent.K2_GetComponentLocation` (`self.BoxD`))))
    (if (`self.InvertBox`)
      (`KismetMaterialLibrary.SetScalarParameterValue` "/Game/ArchitectualSectionTool/Materials/MPC_ArchitecturalParameters.MPC_ArchitecturalParameters" "InvertBox" 1.0)
      (else
        (`KismetMaterialLibrary.SetScalarParameterValue` "/Game/ArchitectualSectionTool/Materials/MPC_ArchitecturalParameters.MPC_ArchitecturalParameters" "InvertBox")))
    (else
      (`KismetMaterialLibrary.SetScalarParameterValue` "/Game/ArchitectualSectionTool/Materials/MPC_ArchitecturalParameters.MPC_ArchitecturalParameters" "ToggleBox"))))