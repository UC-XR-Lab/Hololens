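; Spherical cutout actor for an architectural section tool that drives a cutaway through the MPC_ArchitecturalParameters material parameter collection.
; The construction script scales and sets the opacity of a preview sphere, then writes toggle, centre, radius and invert values to the collection.
; BeginPlay reapplies toggle and invert, and Tick can update centre and radius every frame.
; Events change the radius or switch the cutout on and off at runtime.
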(event `self.ReceiveBeginPlay`
  (`KismetMaterialLibrary.SetScalarParameterValue` "/Game/ArchitectualSectionTool/Materials/MPC_ArchitecturalParameters.MPC_ArchitecturalParameters" "ToggleSphericalCutaway" (`KismetMathLibrary.Conv_BoolToDouble` (`self.ToggleSphericalCutout`)))
  (`KismetMaterialLibrary.SetScalarParameterValue` "/Game/ArchitectualSectionTool/Materials/MPC_ArchitecturalParameters.MPC_ArchitecturalParameters" "InvertSphericalCutaway" (`KismetMathLibrary.Conv_BoolToDouble` (not (`self.InvertSphericalCutout`)))))

(event `self.ReceiveTick`
  (params (DeltaSeconds :type "Float (single-precision)"))
  (if (`self.UpdateEveryFrame`)
    (`KismetMaterialLibrary.SetVectorParameterValue` "/Game/ArchitectualSectionTool/Materials/MPC_ArchitecturalParameters.MPC_ArchitecturalParameters" "SphericalCutawayCentre" (`KismetMathLibrary.Conv_VectorToLinearColor` (`SceneComponent.K2_GetComponentLocation` (`self.Sphere`))))
    (`KismetMaterialLibrary.SetScalarParameterValue` "/Game/ArchitectualSectionTool/Materials/MPC_ArchitecturalParameters.MPC_ArchitecturalParameters" "SphericalCutawayRadius" (`self.Radius`))))

(event `SetRadius`
  (params (Radius :type "Float (double-precision)"))
  (set `self.Radius` Radius)
  (`KismetMaterialLibrary.SetScalarParameterValue` "/Game/ArchitectualSectionTool/Materials/MPC_ArchitecturalParameters.MPC_ArchitecturalParameters" "SphericalCutawayRadius" (`self.Radius`)))

(event `ToggleSphericalCutoutOnOff`
  (if (`self.ToggleSphericalCutout`)
    (`KismetMaterialLibrary.SetScalarParameterValue` "/Game/ArchitectualSectionTool/Materials/MPC_ArchitecturalParameters.MPC_ArchitecturalParameters" "ToggleSphericalCutaway")
    (set `self.ToggleSphericalCutout` false)
    (else
      (`KismetMaterialLibrary.SetScalarParameterValue` "/Game/ArchitectualSectionTool/Materials/MPC_ArchitecturalParameters.MPC_ArchitecturalParameters" "ToggleSphericalCutaway" 1.0)
      (set `self.ToggleSphericalCutout` true))))

(fn `UserConstructionScript`
  (bind _returnvalue (`PrimitiveComponent.CreateDynamicMaterialInstance` (`self.Sphere`) 0 null "None"))
  (`MaterialInstanceDynamic.SetScalarParameterValue` _returnvalue "Opacity" (`self.Opacity`))
  (`SceneComponent.SetWorldScale3D` (`self.Sphere`) (`KismetMathLibrary.Conv_DoubleToVector` (* (`self.Radius`) 0.02)))
  (if (`self.ToggleSphericalCutout`)
    (`KismetMaterialLibrary.SetScalarParameterValue` "/Game/ArchitectualSectionTool/Materials/MPC_ArchitecturalParameters.MPC_ArchitecturalParameters" "ToggleSphericalCutaway" 1.0)
    (`KismetMaterialLibrary.SetScalarParameterValue` "/Game/ArchitectualSectionTool/Materials/MPC_ArchitecturalParameters.MPC_ArchitecturalParameters" "SphericalCutawayRadius" (`self.Radius`))
    (`KismetMaterialLibrary.SetVectorParameterValue` "/Game/ArchitectualSectionTool/Materials/MPC_ArchitecturalParameters.MPC_ArchitecturalParameters" "SphericalCutawayCentre" (`KismetMathLibrary.Conv_VectorToLinearColor` (`SceneComponent.K2_GetComponentLocation` (`self.Sphere`))))
    (if (`self.InvertSphericalCutout`)
      (`KismetMaterialLibrary.SetScalarParameterValue` "/Game/ArchitectualSectionTool/Materials/MPC_ArchitecturalParameters.MPC_ArchitecturalParameters" "InvertSphericalCutaway")
      (else
        (`KismetMaterialLibrary.SetScalarParameterValue` "/Game/ArchitectualSectionTool/Materials/MPC_ArchitecturalParameters.MPC_ArchitecturalParameters" "InvertSphericalCutaway" 1.0)))
    (else
      (`KismetMaterialLibrary.SetScalarParameterValue` "/Game/ArchitectualSectionTool/Materials/MPC_ArchitecturalParameters.MPC_ArchitecturalParameters" "ToggleSphericalCutaway"))))