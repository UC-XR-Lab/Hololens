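; BP_PlanTool is an architectural plan-cut tool that publishes its Plane's height and an on/off flag to MPC_ArchitecturalParameters for materials to read.
; The construction script writes both values and gives the Plane a dynamic material instance with adjustable Opacity.
; Tick rewrites the values when UpdateEveryFrame is set.
; TogglePlanOnOff writes the inverse flag to the collection but reassigns TogglePlan its existing value, so the variable never flips.
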(event `self.ReceiveTick`
  (params (DeltaSeconds :type "Float (single-precision)"))
  (bind (_returnvalue_x _returnvalue_y _returnvalue_z) (`KismetMathLibrary.BreakVector` (`SceneComponent.K2_GetComponentLocation` (`self.Plane`))))
  (if (`self.UpdateEveryFrame`)
    (`KismetMaterialLibrary.SetScalarParameterValue` "/Game/ArchitectualSectionTool/Materials/MPC_ArchitecturalParameters.MPC_ArchitecturalParameters" "PlanHeight" _returnvalue_z)
    (`KismetMaterialLibrary.SetScalarParameterValue` "/Game/ArchitectualSectionTool/Materials/MPC_ArchitecturalParameters.MPC_ArchitecturalParameters" "TogglePlan" (`KismetMathLibrary.Conv_BoolToDouble` (`self.TogglePlan`)))))

(event `TogglePlanOnOff`
  (if (`self.TogglePlan`)
    (`KismetMaterialLibrary.SetScalarParameterValue` "/Game/ArchitectualSectionTool/Materials/MPC_ArchitecturalParameters.MPC_ArchitecturalParameters" "TogglePlan")
    (set `self.TogglePlan` true)
    (else
      (`KismetMaterialLibrary.SetScalarParameterValue` "/Game/ArchitectualSectionTool/Materials/MPC_ArchitecturalParameters.MPC_ArchitecturalParameters" "TogglePlan" 1.0)
      (set `self.TogglePlan` false))))

(fn `UserConstructionScript`
  (bind (_returnvalue_x _returnvalue_y _returnvalue_z) (`KismetMathLibrary.BreakVector` (`SceneComponent.K2_GetComponentLocation` (`self.Plane`))))
  (`|ExecutionSequence`
    (:`then_0`
      (`KismetMaterialLibrary.SetScalarParameterValue` "/Game/ArchitectualSectionTool/Materials/MPC_ArchitecturalParameters.MPC_ArchitecturalParameters" "PlanHeight" _returnvalue_z)
      (`KismetMaterialLibrary.SetScalarParameterValue` "/Game/ArchitectualSectionTool/Materials/MPC_ArchitecturalParameters.MPC_ArchitecturalParameters" "TogglePlan" (`KismetMathLibrary.Conv_BoolToDouble` (`self.TogglePlan`))))
    (:`then_1`
      (bind _returnvalue (`PrimitiveComponent.CreateDynamicMaterialInstance` (`self.Plane`) 0 null "None"))
      (`MaterialInstanceDynamic.SetScalarParameterValue` _returnvalue "Opacity" (`self.Opacity`)))))