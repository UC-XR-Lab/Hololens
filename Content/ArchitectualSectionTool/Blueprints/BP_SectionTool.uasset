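; Architectural section tool actor that publishes one of four section cuts (A to D, chosen by SectionName) to MPC_ArchitecturalParameters.
; It writes the world locations of its two section points and the UseSection toggle to that slot's collection parameters.
; The construction script does this on edit and sets the plane's opacity through a dynamic material instance.
; Tick repeats the write only when UpdateEveryFrame is on, and ToggleUseSection flips the flag.
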(event `self.ReceiveTick`
  (params (DeltaSeconds :type "Float (single-precision)"))
  (if (`self.UpdateEveryFrame`)
    (switch `/Game/ArchitectualSectionTool/Blueprints/SectionNames` (`self.SectionName`)
      (:`NewEnumerator0`
        (`KismetMaterialLibrary.SetVectorParameterValue` "/Game/ArchitectualSectionTool/Materials/MPC_ArchitecturalParameters.MPC_ArchitecturalParameters" "SectionPointA" (`KismetMathLibrary.Conv_VectorToLinearColor` (`SceneComponent.K2_GetComponentLocation` (`self.SectionPointA`))))
        (`KismetMaterialLibrary.SetVectorParameterValue` "/Game/ArchitectualSectionTool/Materials/MPC_ArchitecturalParameters.MPC_ArchitecturalParameters" "SectionPointA1" (`KismetMathLibrary.Conv_VectorToLinearColor` (`SceneComponent.K2_GetComponentLocation` (`self.SectionPointA1`))))
        (`KismetMaterialLibrary.SetScalarParameterValue` "/Game/ArchitectualSectionTool/Materials/MPC_ArchitecturalParameters.MPC_ArchitecturalParameters" "ToggleSectionA" (`KismetMathLibrary.Conv_BoolToDouble` (`self.UseSection`))))
      (:`NewEnumerator1`
        (`KismetMaterialLibrary.SetVectorParameterValue` "/Game/ArchitectualSectionTool/Materials/MPC_ArchitecturalParameters.MPC_ArchitecturalParameters" "SectionPointB" (`KismetMathLibrary.Conv_VectorToLinearColor` (`SceneComponent.K2_GetComponentLocation` (`self.SectionPointA`))))
        (`KismetMaterialLibrary.SetVectorParameterValue` "/Game/ArchitectualSectionTool/Materials/MPC_ArchitecturalParameters.MPC_ArchitecturalParameters" "SectionPointB1" (`KismetMathLibrary.Conv_VectorToLinearColor` (`SceneComponent.K2_GetComponentLocation` (`self.SectionPointA1`))))
        (`KismetMaterialLibrary.SetScalarParameterValue` "/Game/ArchitectualSectionTool/Materials/MPC_ArchitecturalParameters.MPC_ArchitecturalParameters" "ToggleSectionB" (`KismetMathLibrary.Conv_BoolToDouble` (`self.UseSection`))))
      (:`NewEnumerator2`
        (`KismetMaterialLibrary.SetVectorParameterValue` "/Game/ArchitectualSectionTool/Materials/MPC_ArchitecturalParameters.MPC_ArchitecturalParameters" "SectionPointC" (`KismetMathLibrary.Conv_VectorToLinearColor` (`SceneComponent.K2_GetComponentLocation` (`self.SectionPointA`))))
        (`KismetMaterialLibrary.SetVectorParameterValue` "/Game/ArchitectualSectionTool/Materials/MPC_ArchitecturalParameters.MPC_ArchitecturalParameters" "SectionPointC1" (`KismetMathLibrary.Conv_VectorToLinearColor` (`SceneComponent.K2_GetComponentLocation` (`self.SectionPointA1`))))
        (`KismetMaterialLibrary.SetScalarParameterValue` "/Game/ArchitectualSectionTool/Materials/MPC_ArchitecturalParameters.MPC_ArchitecturalParameters" "ToggleSectionC" (`KismetMathLibrary.Conv_BoolToDouble` (`self.UseSection`))))
      (:`NewEnumerator3`
        (`KismetMaterialLibrary.SetVectorParameterValue` "/Game/ArchitectualSectionTool/Materials/MPC_ArchitecturalParameters.MPC_ArchitecturalParameters" "SectionPointD" (`KismetMathLibrary.Conv_VectorToLinearColor` (`SceneComponent.K2_GetComponentLocation` (`self.SectionPointA`))))
        (`KismetMaterialLibrary.SetVectorParameterValue` "/Game/ArchitectualSectionTool/Materials/MPC_ArchitecturalParameters.MPC_ArchitecturalParameters" "SectionPointD1" (`KismetMathLibrary.Conv_VectorToLinearColor` (`SceneComponent.K2_GetComponentLocation` (`self.SectionPointA1`))))
        (`KismetMaterialLibrary.SetScalarParameterValue` "/Game/ArchitectualSectionTool/Materials/MPC_ArchitecturalParameters.MPC_ArchitecturalParameters" "ToggleSectionD" (`KismetMathLibrary.Conv_BoolToDouble` (`self.UseSection`)))))))

(event `ToggleUseSection`
  (if (`self.UseSection`)
    (set `self.UseSection` false)
    (else
      (set `self.UseSection` true))))

(fn `UserConstructionScript`
  (`|ExecutionSequence`
    (:`then_0`
      (switch `/Game/ArchitectualSectionTool/Blueprints/SectionNames` (`self.SectionName`)
        (:`NewEnumerator0`
          (`KismetMaterialLibrary.SetVectorParameterValue` "/Game/ArchitectualSectionTool/Materials/MPC_ArchitecturalParameters.MPC_ArchitecturalParameters" "SectionPointA" (`KismetMathLibrary.Conv_VectorToLinearColor` (`SceneComponent.K2_GetComponentLocation` (`self.SectionPointA`))))
          (`KismetMaterialLibrary.SetVectorParameterValue` "/Game/ArchitectualSectionTool/Materials/MPC_ArchitecturalParameters.MPC_ArchitecturalParameters" "SectionPointA1" (`KismetMathLibrary.Conv_VectorToLinearColor` (`SceneComponent.K2_GetComponentLocation` (`self.SectionPointA1`))))
          (`KismetMaterialLibrary.SetScalarParameterValue` "/Game/ArchitectualSectionTool/Materials/MPC_ArchitecturalParameters.MPC_ArchitecturalParameters" "ToggleSectionA" (`KismetMathLibrary.Conv_BoolToDouble` (`self.UseSection`))))
        (:`NewEnumerator1`
          (`KismetMaterialLibrary.SetVectorParameterValue` "/Game/ArchitectualSectionTool/Materials/MPC_ArchitecturalParameters.MPC_ArchitecturalParameters" "SectionPointB" (`KismetMathLibrary.Conv_VectorToLinearColor` (`SceneComponent.K2_GetComponentLocation` (`self.SectionPointA`))))
          (`KismetMaterialLibrary.SetVectorParameterValue` "/Game/ArchitectualSectionTool/Materials/MPC_ArchitecturalParameters.MPC_ArchitecturalParameters" "SectionPointB1" (`KismetMathLibrary.Conv_VectorToLinearColor` (`SceneComponent.K2_GetComponentLocation` (`self.SectionPointA1`))))
          (`KismetMaterialLibrary.SetScalarParameterValue` "/Game/ArchitectualSectionTool/Materials/MPC_ArchitecturalParameters.MPC_ArchitecturalParameters" "ToggleSectionB" (`KismetMathLibrary.Conv_BoolToDouble` (`self.UseSection`))))
        (:`NewEnumerator2`
          (`KismetMaterialLibrary.SetVectorParameterValue` "/Game/ArchitectualSectionTool/Materials/MPC_ArchitecturalParameters.MPC_ArchitecturalParameters" "SectionPointC" (`KismetMathLibrary.Conv_VectorToLinearColor` (`SceneComponent.K2_GetComponentLocation` (`self.SectionPointA`))))
          (`KismetMaterialLibrary.SetVectorParameterValue` "/Game/ArchitectualSectionTool/Materials/MPC_ArchitecturalParameters.MPC_ArchitecturalParameters" "SectionPointC1" (`KismetMathLibrary.Conv_VectorToLinearColor` (`SceneComponent.K2_GetComponentLocation` (`self.SectionPointA1`))))
          (`KismetMaterialLibrary.SetScalarParameterValue` "/Game/ArchitectualSectionTool/Materials/MPC_ArchitecturalParameters.MPC_ArchitecturalParameters" "ToggleSectionC" (`KismetMathLibrary.Conv_BoolToDouble` (`self.UseSection`))))
        (:`NewEnumerator3`
          (`KismetMaterialLibrary.SetVectorParameterValue` "/Game/ArchitectualSectionTool/Materials/MPC_ArchitecturalParameters.MPC_ArchitecturalParameters" "SectionPointD" (`KismetMathLibrary.Conv_VectorToLinearColor` (`SceneComponent.K2_GetComponentLocation` (`self.SectionPointA`))))
          (`KismetMaterialLibrary.SetVectorParameterValue` "/Game/ArchitectualSectionTool/Materials/MPC_ArchitecturalParameters.MPC_ArchitecturalParameters" "SectionPointD1" (`KismetMathLibrary.Conv_VectorToLinearColor` (`SceneComponent.K2_GetComponentLocation` (`self.SectionPointA1`))))
          (`KismetMaterialLibrary.SetScalarParameterValue` "/Game/ArchitectualSectionTool/Materials/MPC_ArchitecturalParameters.MPC_ArchitecturalParameters" "ToggleSectionD" (`KismetMathLibrary.Conv_BoolToDouble` (`self.UseSection`))))))
    (:`then_1`
      (bind _returnvalue (`PrimitiveComponent.CreateDynamicMaterialInstance` (`self.Plane`) 0 null "None"))
      (`MaterialInstanceDynamic.SetScalarParameterValue` _returnvalue "Opacity" (`self.Opacity`)))))