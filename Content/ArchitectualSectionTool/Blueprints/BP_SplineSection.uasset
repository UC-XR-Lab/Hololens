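; Spline-driven section actor for an architectural section tool that feeds a cut shape to materials through MPC_ArchitecturalParameters.
; The construction script places two boxes offset along the right vector of spline points 0 and 3.
; It writes the box and four spline point world positions as six vector parameters, plus spline toggle and middle-invert scalars.
; Tick repeats those parameter writes when UpdateEveryFrame is on, without repositioning the boxes.
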(event `self.ReceiveTick`
  (params (DeltaSeconds :type "Float (single-precision)"))
  (if (`self.UpdateEveryFrame`)
    (`KismetMaterialLibrary.SetVectorParameterValue` "/Game/ArchitectualSectionTool/Materials/MPC_ArchitecturalParameters.MPC_ArchitecturalParameters" "SplinePoint0" (`KismetMathLibrary.Conv_VectorToLinearColor` (`SceneComponent.K2_GetComponentLocation` (`self.Box`))))
    (`KismetMaterialLibrary.SetVectorParameterValue` "/Game/ArchitectualSectionTool/Materials/MPC_ArchitecturalParameters.MPC_ArchitecturalParameters" "SplinePoint1" (`KismetMathLibrary.Conv_VectorToLinearColor` (`SplineComponent.GetLocationAtSplinePoint` (`self.Spline`) 0 "World")))
    (`KismetMaterialLibrary.SetVectorParameterValue` "/Game/ArchitectualSectionTool/Materials/MPC_ArchitecturalParameters.MPC_ArchitecturalParameters" "SplinePoint2" (`KismetMathLibrary.Conv_VectorToLinearColor` (`SplineComponent.GetLocationAtSplinePoint` (`self.Spline`) 1 "World")))
    (`KismetMaterialLibrary.SetVectorParameterValue` "/Game/ArchitectualSectionTool/Materials/MPC_ArchitecturalParameters.MPC_ArchitecturalParameters" "SplinePoint3" (`KismetMathLibrary.Conv_VectorToLinearColor` (`SplineComponent.GetLocationAtSplinePoint` (`self.Spline`) 2 "World")))
    (`KismetMaterialLibrary.SetVectorParameterValue` "/Game/ArchitectualSectionTool/Materials/MPC_ArchitecturalParameters.MPC_ArchitecturalParameters" "SplinePoint4" (`KismetMathLibrary.Conv_VectorToLinearColor` (`SplineComponent.GetLocationAtSplinePoint` (`self.Spline`) 3 "World")))
    (`KismetMaterialLibrary.SetVectorParameterValue` "/Game/ArchitectualSectionTool/Materials/MPC_ArchitecturalParameters.MPC_ArchitecturalParameters" "SplinePoint5" (`KismetMathLibrary.Conv_VectorToLinearColor` (`SceneComponent.K2_GetComponentLocation` (`self.Box1`))))
    (if (`self.ToggleSplineSection`)
      (`KismetMaterialLibrary.SetScalarParameterValue` "/Game/ArchitectualSectionTool/Materials/MPC_ArchitecturalParameters.MPC_ArchitecturalParameters" "ToggleSpline" 1.0)
      (if (`self.InvertMiddle`)
        (`KismetMaterialLibrary.SetScalarParameterValue` "/Game/ArchitectualSectionTool/Materials/MPC_ArchitecturalParameters.MPC_ArchitecturalParameters" "InvertMiddle" 1.0)
        (else
          (`KismetMaterialLibrary.SetScalarParameterValue` "/Game/ArchitectualSectionTool/Materials/MPC_ArchitecturalParameters.MPC_ArchitecturalParameters" "InvertMiddle")))
      (else
        (`KismetMaterialLibrary.SetScalarParameterValue` "/Game/ArchitectualSectionTool/Materials/MPC_ArchitecturalParameters.MPC_ArchitecturalParameters" "ToggleSpline")))))

(fn `UserConstructionScript`
  (bind _spline (`self.Spline`))
  (bind _spline_2 (`self.Spline`))
  (`SceneComponent.K2_SetWorldLocation` (`self.Box`) (+ (.location (`SplineComponent.GetTransformAtSplinePoint` _spline 0 "World" false)) (* (`SplineComponent.GetRightVectorAtSplinePoint` _spline 0 "World") 100.0)) false false)
  (`SceneComponent.K2_SetWorldLocation` (`self.Box1`) (+ (.location (`SplineComponent.GetTransformAtSplinePoint` _spline_2 3 "World" false)) (* (`SplineComponent.GetRightVectorAtSplinePoint` _spline_2 3 "World") 100.0)) false false)
  (if (`self.ToggleSplineSection`)
    (`KismetMaterialLibrary.SetScalarParameterValue` "/Game/ArchitectualSectionTool/Materials/MPC_ArchitecturalParameters.MPC_ArchitecturalParameters" "ToggleSpline" 1.0)
    (`KismetMaterialLibrary.SetVectorParameterValue` "/Game/ArchitectualSectionTool/Materials/MPC_ArchitecturalParameters.MPC_ArchitecturalParameters" "SplinePoint0" (`KismetMathLibrary.Conv_VectorToLinearColor` (`SceneComponent.K2_GetComponentLocation` (`self.Box`))))
    (`KismetMaterialLibrary.SetVectorParameterValue` "/Game/ArchitectualSectionTool/Materials/MPC_ArchitecturalParameters.MPC_ArchitecturalParameters" "SplinePoint1" (`KismetMathLibrary.Conv_VectorToLinearColor` (`SplineComponent.GetLocationAtSplinePoint` (`self.Spline`) 0 "World")))
    (`KismetMaterialLibrary.SetVectorParameterValue` "/Game/ArchitectualSectionTool/Materials/MPC_ArchitecturalParameters.MPC_ArchitecturalParameters" "SplinePoint2" (`KismetMathLibrary.Conv_VectorToLinearColor` (`SplineComponent.GetLocationAtSplinePoint` (`self.Spline`) 1 "World")))
    (`KismetMaterialLibrary.SetVectorParameterValue` "/Game/ArchitectualSectionTool/Materials/MPC_ArchitecturalParameters.MPC_ArchitecturalParameters" "SplinePoint3" (`KismetMathLibrary.Conv_VectorToLinearColor` (`SplineComponent.GetLocationAtSplinePoint` (`self.Spline`) 2 "World")))
    (`KismetMaterialLibrary.SetVectorParameterValue` "/Game/ArchitectualSectionTool/Materials/MPC_ArchitecturalParameters.MPC_ArchitecturalParameters" "SplinePoint4" (`KismetMathLibrary.Conv_VectorToLinearColor` (`SplineComponent.GetLocationAtSplinePoint` (`self.Spline`) 3 "World")))
    (`KismetMaterialLibrary.SetVectorParameterValue` "/Game/ArchitectualSectionTool/Materials/MPC_ArchitecturalParameters.MPC_ArchitecturalParameters" "SplinePoint5" (`KismetMathLibrary.Conv_VectorToLinearColor` (`SceneComponent.K2_GetComponentLocation` (`self.Box1`))))
    (if (`self.InvertMiddle`)
      (`KismetMaterialLibrary.SetScalarParameterValue` "/Game/ArchitectualSectionTool/Materials/MPC_ArchitecturalParameters.MPC_ArchitecturalParameters" "InvertMiddle" 1.0)
      (else
        (`KismetMaterialLibrary.SetScalarParameterValue` "/Game/ArchitectualSectionTool/Materials/MPC_ArchitecturalParameters.MPC_ArchitecturalParameters" "InvertMiddle")))
    (else
      (`KismetMaterialLibrary.SetScalarParameterValue` "/Game/ArchitectualSectionTool/Materials/MPC_ArchitecturalParameters.MPC_ArchitecturalParameters" "ToggleSpline"))))