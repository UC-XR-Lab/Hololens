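; An AR actor that turns on QR code detection and responds to tracked code updates.
; A short timer after BeginPlay enables QR capture, and an ARTrackableNotify component reports tracked geometry; the add handler only casts.
; Each QR update resets the Board actor to an identity transform, ignoring the code's pose, and draws a debug box from the code's transform and estimated size.
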(event `self.ReceiveBeginPlay`
  (`KismetSystemLibrary.K2_SetTimerDelegate` (delegate `OnTimerDelay`) 5.0))

(event `OnTimerDelay`
  (`ARBlueprintLibrary.ToggleARCapture` true "QRCode"))

(event `self.ARTrackableNotify.OnAddTrackedGeometry`
  (params (TrackedGeometry :type "ARTrackedGeometry Object Reference"))
  (bind _asartracked_qrcode (cast `ARTrackedQRCode` TrackedGeometry)))

(event `self.ARTrackableNotify.OnUpdateTrackedGeometry`
  (params (TrackedGeometry :type "ARTrackedGeometry Object Reference"))
  (bind _asartracked_qrcode (cast `ARTrackedQRCode` TrackedGeometry))
  (bind _returnvalue (`GameplayStatics.GetActorOfClass` "/Game/Blueprints/Board.Board_C"))
  (`self.K2_SetActorTransform` _returnvalue (`KismetMathLibrary.MakeTransform` (0.0 0.0 0.0)) false false)
  (bind _returnvalue_2 (`ARTrackedGeometry.GetLocalToWorldTransform` _asartracked_qrcode))
  (bind (_x _y) (`KismetMathLibrary.BreakVector2D` (`ARTrackedImage.GetEstimateSize` _asartracked_qrcode)))
  (bind _returnvalue_3 (/ (`KismetMathLibrary.MakeVector` 0.0 _x _y) 2.0))
  (`KismetSystemLibrary.DrawDebugBox` (`KismetMathLibrary.TransformLocation` _returnvalue_2 _returnvalue_3) _returnvalue_3 (struct) (`KismetMathLibrary.TransformRotation` _returnvalue_2)))

(fn `UserConstructionScript`)