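; Button actor that pages through instruction lines on the Board actor with Next and Back UXT pressable buttons.
; Tick polls both child-actor buttons, using flags so each press steps the shared index only once.
; Each press re-reads a text file at a hard-coded Z: drive path and sends that line to the Board, without bounds checks.
; An alternative DataTable lookup is left disconnected and never runs.
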(event `self.ReceiveBeginPlay`
  ;[1 1 1] Initialization: Fetch and store a reference to the Board actor at game start.
  (bind _returnvalue (`GameplayStatics.GetActorOfClass` "/Game/Blueprints/Board.Board_C"))
  (set `self.Boardref` _returnvalue))

(event `self.ReceiveTick`
  (params (DeltaSeconds :type "Float (single-precision)"))
  (bind _int (`self.int`))
  (`|ExecutionSequence`
    (:`then_0`
      (bind _asuxt_pressable_button_actor (cast `UxtPressableButtonActor` (`ChildActorComponent.ChildActor` (`self.Next Button`))))
      (if (`|EnumEquality` (`UxtPressableButtonComponent.GetState` (`UxtBasePressableButtonActor.ButtonComponent` _asuxt_pressable_button_actor)) "Pressed")
        (if (not (`self.pressedN`))
          (set `self.pressedN` true)
          (bind _result (`/Engine/EditorBlueprintResources/StandardMacros.IncrementInt` _int)
            (:`  `
              (`KismetSystemLibrary.PrintString` "Hello")
              (`/Game/Blueprints/Board.set text` (`self.Boardref`) (`KismetTextLibrary.Conv_StringToText` (`|GetArrayItem` (`FileSDKBPLibrary.ReadLinesFromFile` "Z:\\XRLab\\instructions.txt") _result))))))
        (elif (`self.pressedN`)
          (set `self.pressedN` false))))
    (:`then_1`
      (bind _asuxt_pressable_button_actor_2 (cast `UxtPressableButtonActor` (`ChildActorComponent.ChildActor` (`self.Back Button`))))
      (if (`|EnumEquality` (`UxtPressableButtonComponent.GetState` (`UxtBasePressableButtonActor.ButtonComponent` _asuxt_pressable_button_actor_2)) "Pressed")
        (if (not (`self.pressedB`))
          (set `self.pressedB` true)
          (bind _result_2 (`/Engine/EditorBlueprintResources/StandardMacros.DecrementInt` _int)
            (:`  `
              (`KismetSystemLibrary.PrintString` "121212")
              (`/Game/Blueprints/Board.set text` (`self.Boardref`) (`KismetTextLibrary.Conv_StringToText` (`|GetArrayItem` (`FileSDKBPLibrary.ReadLinesFromFile` "Z:\\XRLab\\instructions.txt") _result_2))))))
        (elif (`self.pressedB`)
          (set `self.pressedB` false))))))

(fn `UserConstructionScript`)